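; FMOD ambient sound actor that fades the Player and Shadow parameters of the OST music event.
; SwapToPlayer, SwapToShadow and SwapToBoth set two flags choosing which parameters are active, with both enabled on BeginPlay.
; Each Tick, LerpParamTo steps each parameter linearly toward 1 or 0 on the first OST instance found, with FadeStrength as the full fade time in seconds.
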(event EventBeginPlay
  (CallFunction|SwaptoBoth))

(event EventTick
  (params (DeltaSeconds :type Float%20%28single-precision%29))
  (CallFunction|LerpParamto (Variables|Default|GetIsPlayer) (Variables|Default|GetPlayer))
  (CallFunction|LerpParamto (Variables|Default|GetIsShadow) (Variables|Default|GetShadow)))

(fn ConstructionScript)

(fn LerpParamto
  (params (LerpTo1 :type Boolean) (ParamName :type Name))
  (bind _returnvalue (Utilities|Time|GetWorldDeltaSeconds))
  (bind _fadestrength (Variables|Default|GetFadeStrength))
  (bind _returnvalue_2 (Math|Float|SafeDivide _returnvalue _fadestrength))
  (bind _returnvalue_3 (Class|FMODBlueprintStatics|FindEventInstances "/Game/FMOD/Events/OST.OST"))
  (bind _returnvalue_4 (Class|FMODBlueprintStatics|EventInstanceGetParameter (Utilities|Array|Get(acopy) _returnvalue_3) ParamName))
  (if LerpTo1
    (Class|FMODBlueprintStatics|EventInstanceSetParameter (Utilities|Array|Get(acopy) _returnvalue_3) ParamName (Math|Float|Clamp(Float) (+ _returnvalue_2 _returnvalue_4)))
    (else
      (Class|FMODBlueprintStatics|EventInstanceSetParameter (Utilities|Array|Get(acopy) _returnvalue_3) ParamName (Math|Float|Clamp(Float) (- _returnvalue_4 _returnvalue_2))))))

(fn SwaptoBoth
  (Variables|Default|SetIsPlayer true)
  (Variables|Default|SetIsShadow true))

(fn SwaptoPlayer
  (Variables|Default|SetIsPlayer true)
  (Variables|Default|SetIsShadow false))

(fn SwaptoShadow
  (Variables|Default|SetIsPlayer false)
  (Variables|Default|SetIsShadow true))