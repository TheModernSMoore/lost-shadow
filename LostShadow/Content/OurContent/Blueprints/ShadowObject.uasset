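; A block the player can push or pull, which also computes the outline of the shadow it casts on a wall.
; Hits from the player snap to an X or Y direction, pass trace checks, then attach the player while a timeline slides the block.
; Each tick, line traces from PsudeoLightSource project lit silhouette vertices onto the wall.
; These 2D points are sorted angularly around their centroid, with UpdatePolygon flagging changes.
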(event Custom|Push
  (Variables|Default|SetcurrentLocation (Transformation|GetActorLocation))
  (bind _position (Timeline|MoveBlock😎 PlayFromStart)
    (:Update
      (Transformation|SetActorRelativeLocation (+ (Variables|Default|GetcurrentLocation) (* _position (Variables|Default|GetpushDirection) (Variables|Default|GetTRAVEL_DISTANCE)))))
    (:Finished
      (CallFunction|StopPushing))))

(event Custom|Stop%20Pushing
  (bind _returnvalue (Game|GetPlayerCharacter 0))
  (Pawn|Components|CharacterMovement|SetMovementMode (Variables|/Script/Engine.Character|GetCharacterMovement _returnvalue) "MOVE_Walking" 0)
  (Transformation|DetachFromActor _returnvalue "KeepWorld" "KeepWorld" "KeepWorld")
  (bind _asbp_third_person_character (Utilities|Casting|CastToBP_ThirdPersonCharacter _returnvalue))
  (Variables|/Game/ThirdPerson/Blueprints/BP_ThirdPersonCharacter.BP_ThirdPersonCharacter_C|SetPush/PullState _asbp_third_person_character false))

(event Custom|Pull
  (Variables|Default|SetcurrentLocation (Transformation|GetActorLocation))
  (bind _position (Timeline|Timeline PlayFromStart)
    (:Update
      (Transformation|SetActorRelativeLocation (+ (Variables|Default|GetcurrentLocation) (* _position (Variables|Default|GetpushDirection) (* (Variables|Default|GetTRAVEL_DISTANCE) -1.0)))))
    (:Finished
      (CallFunction|StopPushing))))

(event EventBeginPlay
  (bind _vertices (Class|KismetProceduralMeshLibrary|GetSectionfromStaticMesh (Variables|/Script/Engine.StaticMeshComponent|GetStaticMesh (Variables|Default|GetCube))))
  (Variables|Default|SetMesh%20Vertices _vertices))

(event Collision|EventActorBeginOverlap
  (params (OtherActor :type Actor%20Object%20Reference)))

(event EventTick
  (params (DeltaSeconds :type Float%20%28single-precision%29))
  (bind _cube (Variables|Default|GetCube))
  (bind _returnvalue (Transformation|GetWorldLocation _cube))
  (bind _outactors (Actor|GetAllActorsOfClass "/Game/ThirdPerson/Blueprints/Shadow_Character.Shadow_Character_C"))
  (bind _outactors_2 (Actor|GetAllActorsOfClass "/Game/OurContent/Blueprints/PsudeoLightSource.PsudeoLightSource_C"))
  (bind (_outhit _returnvalue_2) (Collision|LineTraceByChannel (+ (* (Math|Vector|GetUnitDirection(Vector) (Transformation|GetWorldLocation (Variables|/Game/OurContent/Blueprints/PsudeoLightSource.PsudeoLightSource_C|GetSphere (Utilities|Array|Get(acopy) _outactors_2))) _returnvalue) 1e+02) _returnvalue) (+ (* (Math|Vector|GetUnitDirection(Vector) (Transformation|GetWorldLocation (Variables|/Game/OurContent/Blueprints/PsudeoLightSource.PsudeoLightSource_C|GetSphere (Utilities|Array|Get(acopy) _outactors_2))) _returnvalue) 2e+05) (Transformation|GetWorldLocation (Variables|/Game/OurContent/Blueprints/PsudeoLightSource.PsudeoLightSource_C|GetSphere (Utilities|Array|Get(acopy) _outactors_2)))) "TraceTypeQuery3" true 0 "ForOneFrame" true "(R=0.168398,G=0.410070,B=1.000000,A=1.000000)" "(R=1.000000,G=0.972759,B=0.323792,A=1.000000)"))
  (if _returnvalue_2
    (bind _output_get (Variables|Default|SetobjectCenterPoint:%29 (Math|Vector2D|MakeVector2D (.Z (Math|Vector|BreakVector (.Location (Collision|BreakHitResult _outhit)))) (.Y (Math|Vector|BreakVector (.Location (Collision|BreakHitResult _outhit))))))))
  (Variables|Default|SetlightSourceWorldLocation (Transformation|GetWorldLocation (Variables|/Game/OurContent/Blueprints/PsudeoLightSource.PsudeoLightSource_C|GetSphere (Utilities|Array|Get(acopy) _outactors_2))))
  (for _array_element (Variables|Default|GetMesh%20Vertices)
    (Variables|Default|SetverticeWorldLocation (Math|Transform|TransformLocation (Transformation|GetWorldTransform (Variables|Default|GetCube)) _array_element))
    (Variables|Default|SetunitVectorSphereToVertice (Math|Vector|GetUnitDirection(Vector) (Variables|Default|GetlightSourceWorldLocation) (Variables|Default|GetverticeWorldLocation)))
    ;[1 1 1] Line trace from sphere to slightly infront of vertice - reason is to find what vertices are on the "lit" sides of object
    (bind _returnvalue_3 (Collision|LineTraceByChannel (- (Variables|Default|GetverticeWorldLocation) (* (Variables|Default|GetunitVectorSphereToVertice) 5.0)) (+ (Variables|Default|GetlightSourceWorldLocation) (* (Variables|Default|GetunitVectorSphereToVertice) 13.0)) "TraceTypeQuery4" false 0 "None" false "(R=1.000000,G=0.542473,B=0.335917,A=1.000000)" "(R=0.237762,G=0.735597,B=1.000000,A=1.000000)"))
    (if (not _returnvalue_3)
      (bind _isedge (CallFunction|CheckifEdge (Variables|Default|GetverticeWorldLocation)))
      (if _isedge
        (bind _outactors_3 (Actor|GetAllActorsOfClass "/Game/OurContent/Blueprints/ShadowWallCollision.ShadowWallCollision_C"))
        ;[1 1 1] Line trace from vertice in direction of sphere to vertice - reason is to find where edge vertices hit the wall and get the location to create shadow objects
        (bind (_outhit_2 _returnvalue_4) (Collision|LineTraceByChannel (Variables|Default|GetverticeWorldLocation) (+ (Variables|Default|GetverticeWorldLocation) (* (Variables|Default|GetunitVectorSphereToVertice) (Variables|Default|GetVERTICE_TO_WALL_LINE_TRACE_DISTANCE))) "TraceTypeQuery3" false _outactors_3 "ForOneFrame" true "(R=1.000000,G=0.148814,B=0.128918,A=1.000000)" "(R=0.131713,G=0.099750,B=1.000000,A=1.000000)" 1.0))
        (if _returnvalue_4
          (Utilities|Array|Add (Variables|Default|GetTemp%20Points%20Hit%20Locations) (.Location (Collision|BreakHitResult _outhit_2)))
          (Utilities|Array|Add (Variables|Default|GetTemp%202D%20Point%20Locations) (Math|Vector2D|MakeVector2D (.Z (Math|Vector|BreakVector (.Location (Collision|BreakHitResult _outhit_2)))) (.Y (Math|Vector|BreakVector (.Location (Collision|BreakHitResult _outhit_2))))))))))
  (Variables|Default|SetLatest%20Point%20Locations (Variables|Default|GetTemp%20Points%20Hit%20Locations))
  (Utilities|Array|Clear (Variables|Default|GetTemp%20Points%20Hit%20Locations))
  (Variables|Default|SetupdatePolygon? false)
  (if (== (Utilities|Array|Length (Variables|Default|GetTemp%202D%20Point%20Locations)) (Utilities|Array|Length (Variables|Default|GetLatest%202D%20Point%20Locations)))
    (for (_array_element_2 _array_index) (Variables|Default|GetLatest%202D%20Point%20Locations)
      (if (not (Utilities|Operators|EqualEqual _array_element_2 (Utilities|Array|Get(acopy) (Variables|Default|GetTemp%202D%20Point%20Locations) _array_index) 0.05))
        (Variables|Default|SetupdatePolygon? true)))
    (else
      (Variables|Default|SetupdatePolygon? true)))
  (bind _output_get_2 (Variables|Default|SetLatest%202D%20Point%20Locations (Variables|Default|GetTemp%202D%20Point%20Locations)))
  (bind _sorted_2d (CallFunction|BrocksFunction _output_get_2))
  (Variables|Default|SetLatest%202D%20Point%20Locations _sorted_2d)
  (Utilities|Array|Clear (Variables|Default|GetTemp%202D%20Point%20Locations)))

(event Collision|EventHit
  (params (MyComp :type Primitive%20Component%20Object%20Reference) (Other :type Actor%20Object%20Reference) (OtherComp :type Primitive%20Component%20Object%20Reference) (bSelfMoved :type Boolean) (HitLocation :type Vector :default "0, 0, 0") (HitNormal :type Vector :default "0, 0, 0") (NormalImpulse :type Vector :default "0, 0, 0") (Hit :type Hit%20Result%20Structure%20%28by%20ref%29))
  (bind _returnvalue (Transformation|GetActorForwardVector Other))
  (bind _returnvalue_2 (Game|GetPlayerCharacter 0))
  (bind (_x _y) (Math|Vector|BreakVector _returnvalue))
  (bind _returnvalue_3 (Math|Float|Absolute(Float) _x))
  (bind _returnvalue_4 (Math|Float|Absolute(Float) _y))
  (if (== (Game|GetPlayerCharacter 0) Other)
    (Math|Float|CompareFloat _returnvalue_3 _returnvalue_4
      (:>
        (if (> _returnvalue_3 0.8)
          (Variables|Default|SetpushDirection (Math|Vector|MakeVector (Math|Conversions|ToFloat(Integer) (Math|Float|Round _x)) 0.0 0.0))
          (bind _canpush (CallFunction|CanPush :!label _label))
          (if _canpush
            (bind _asbp_third_person_character (Utilities|Casting|CastToBP_ThirdPersonCharacter _returnvalue_2)
              (:then
                (Variables|/Game/ThirdPerson/Blueprints/BP_ThirdPersonCharacter.BP_ThirdPersonCharacter_C|SetPush/PullState _asbp_third_person_character true))
              (:CastFailed
                _))
            (Pawn|Components|CharacterMovement|DisableMovement (Variables|/Script/Engine.Character|GetCharacterMovement _returnvalue_2))
            (Transformation|AttachActorToActor _returnvalue_2 self "None" "KeepWorld" "KeepWorld" "KeepWorld" true)
            (bind _outactors (Actor|GetAllActorsOfClass "/Game/ThirdPerson/Blueprints/BP_ThirdPersonCharacter.BP_ThirdPersonCharacter_C"))
            (if (Variables|/Game/ThirdPerson/Blueprints/BP_ThirdPersonCharacter.BP_ThirdPersonCharacter_C|GetisPulling? (Utilities|Array|Get(acopy) _outactors))
              (CallFunction|Pull)
              (else
                (CallFunction|Push))))
          (else
            (Variables|Default|SetpushDirection "0, 0, 0" :!label _label_2))))
      (:==
        (goto _label_2))
      (:<
        (if (> _returnvalue_4 0.8)
          (Variables|Default|SetpushDirection (Math|Vector|MakeVector 0.0 (Math|Conversions|ToFloat(Integer) (Math|Float|Round _y)) 0.0))
          (goto _label)
          (else
            (goto _label_2)))))))

(fn ConstructionScript)

(fn CheckifEdge
  (params (Vertice :type Vector))
  (bind _outactors (Actor|GetAllActorsOfClass "/Game/OurContent/Blueprints/PsudeoLightSource.PsudeoLightSource_C"))
  (Variables|Default|SetlightSourceWorldLocation (Transformation|GetWorldLocation (Variables|/Game/OurContent/Blueprints/PsudeoLightSource.PsudeoLightSource_C|GetSphere (Utilities|Array|Get(acopy) _outactors))))
  (Variables|Default|SetunitVectorSphereToVertice (Math|Vector|GetUnitDirection(Vector) (Variables|Default|GetlightSourceWorldLocation) Vertice))
  (Variables|Components|SetcheckEdgeStartLocation (+ (Variables|Default|GetlightSourceWorldLocation) (* (Variables|Default|GetunitVectorSphereToVertice) (Variables|Default|GetSPHERE_RADIUS+Some))))
  ;[1 1 1] Check for up/down and left/right
  (for _array_element (Variables|Default|GetAXIS_OF_ROTATION)
    (Utilities|FlowControl|Sequence
      (:then_0
        ;[1 1 1] Line trace slightly up/right
        (bind _returnvalue (Collision|LineTraceByChannel (Variables|Components|GetcheckEdgeStartLocation) (+ (* (Math|Vector|RotateVectorAroundAxis (Variables|Default|GetunitVectorSphereToVertice) 1.0 _array_element) (Variables|Default|GetCHECK_IF_EDGE_LINE_TRACE_DISTANCE)) Vertice) "TraceTypeQuery4" false 0 "None" false "(R=1.000000,G=0.915755,B=0.007022,A=1.000000)" "(R=0.856275,G=0.267401,B=1.000000,A=1.000000)" 1.0))
        (if (not _returnvalue)
          (return true)))
      (:then_1
        ;[1 1 1] Line trace slightly down/left
        (bind _returnvalue_2 (Collision|LineTraceByChannel (Variables|Components|GetcheckEdgeStartLocation) (+ (* (Math|Vector|RotateVectorAroundAxis (Variables|Default|GetunitVectorSphereToVertice) -1.0 _array_element) (Variables|Default|GetCHECK_IF_EDGE_LINE_TRACE_DISTANCE)) Vertice) "TraceTypeQuery4" false 0 "None" false "(R=0.796589,G=1.000000,B=0.888543,A=1.000000)" "(R=0.365774,G=1.000000,B=0.446747,A=1.000000)" 1.0))
        (if (not _returnvalue_2)
          (return true)))
      (:then_2
        (return false)))))

(fn BrocksFunction
  (params (2d%20UNSORTED :type Array%20of%20Vector%202D%20Structures))
  (Variables|Default|Settemp%20unsorted%202d%20Array 2d%20UNSORTED)
  (bind _centerpoint__ (CallFunction|APPgETCUNETERPOINT!! (Variables|Default|Gettemp%20unsorted%202d%20Array)))
  (Variables|Default|SetCenterPoint _centerpoint__)
  (for (_array_element _array_index) (Variables|Default|Gettemp%20unsorted%202d%20Array)
    (for (_array_element_2 _array_index_2) (Variables|Default|Gettemp%20unsorted%202d%20Array)
      (bind _boolean (CallFunction|AppGetLessYeah _array_element _array_element_2 _centerpoint__))
      (if (not _boolean)
        (Utilities|Array|Swap (Variables|Default|Gettemp%20unsorted%202d%20Array) _array_index_2 _array_index))))
  (return (Variables|Default|Gettemp%20unsorted%202d%20Array)))

(fn AppGetLessYeah
  (params (A :type Vector%202D%20Structure) (B :type Vector%202D%20Structure) (Center%20Point :type Vector%202D%20Structure))
  (bind _returnvalue (- (.x A) (.x Center%20Point)))
  (bind _returnvalue_2 (- (.y B) (.y Center%20Point)))
  (bind _returnvalue_3 (- (.x B) (.x Center%20Point)))
  (bind _returnvalue_4 (- (.y A) (.y Center%20Point)))
  (bind _returnvalue_5 (* _returnvalue _returnvalue_2))
  (bind _returnvalue_6 (* _returnvalue_3 _returnvalue_4))
  (bind _returnvalue_7 (- _returnvalue_5 _returnvalue_6))
  (if (and (>= (- (.x A) (.x Center%20Point)) 0.0) (< (- (.x B) (.x Center%20Point)) 0.0))
    (return true)
    (elif (and (< (- (.x A) (.x Center%20Point)) 0.0) (>= (- (.x B) (.x Center%20Point)) 0.0))
      (return false)
      (elif (and (== (- (.x A) (.x Center%20Point)) 0.0) (== (- (.x B) (.x Center%20Point)) 0.0))
        (if (or (>= (- (.y A) (.y Center%20Point)) 0.0) (>= (.y B) (.y Center%20Point)))
          (return (> (.y A) (.y B)))
          (else
            (return (> (.y B) (.y A)))))
        (elif (< _returnvalue_7 0.0)
          (return true)
          (elif (> _returnvalue_7 0.0)
            (return false)
            (else
              (return (> (+ (Math|Float|Square (- (.x A) (.x Center%20Point))) (Math|Float|Square (- (.y A) (.y Center%20Point)))) (+ (Math|Float|Square (- (.x B) (.x Center%20Point))) (Math|Float|Square (- (.y B) (.y Center%20Point)))))))))))))

(fn APPgETCUNETERPOINT!!
  (params (points :type Array%20of%20Vector%202D%20Structures))
  (bind _returnvalue (Utilities|Array|Length points))
  (Variables|Default|SetpointsSum "")
  (for _array_element points
    (Variables|Default|SetpointsSum (+ _array_element (Variables|Default|GetpointsSum))))
  (return (Math|Vector2D|MakeVector2D (/ (.x (Variables|Default|GetpointsSum)) _returnvalue) (/ (.y (Variables|Default|GetpointsSum)) _returnvalue))))

(fn CanPush
  (bind _boxextent (Collision|GetActorBounds false false))
  (bind _returnvalue (Transformation|GetActorLocation))
  (bind _boxextent_2 (Collision|GetActorBounds false false))
  (bind _returnvalue_2 (Transformation|GetActorLocation))
  (bind _returnvalue_3 (Actor|GetActorOfClass "/Game/ThirdPerson/Blueprints/BP_ThirdPersonCharacter.BP_ThirdPersonCharacter_C"))
  (if (not (AI|Components|NavMovement|IsFalling (Variables|/Script/Engine.Character|GetCharacterMovement _returnvalue_3)))
    (bind (_outhit _returnvalue_4) (Collision|LineTraceByChannel (Transformation|GetActorLocation _returnvalue_3) (+ (Transformation|GetActorLocation _returnvalue_3) (* (Transformation|GetActorForwardVector _returnvalue_3) 75.0)) "TraceTypeQuery4" true (Utilities|Array|MakeArray _returnvalue_3) "ForOneFrame" false))
    (if _returnvalue_4
      (if (== (.HitActor (Collision|BreakHitResult _outhit)) self)
        (bind _outactors (Actor|GetAllActorsOfClass "/Game/ThirdPerson/Blueprints/BP_ThirdPersonCharacter.BP_ThirdPersonCharacter_C"))
        (if (Variables|/Game/ThirdPerson/Blueprints/BP_ThirdPersonCharacter.BP_ThirdPersonCharacter_C|GetisPulling? (Utilities|Array|Get(acopy) _outactors))
          (bind _returnvalue_5 (Collision|BoxTraceByChannel _returnvalue_2 (+ (* (* (Transformation|GetActorForwardVector _returnvalue_3) -1.0) 1.5e+02) _returnvalue_2) (Math|Vector|MakeVector (.x _boxextent_2) (.y _boxextent_2) (* (.z _boxextent_2) 0.9)) "0, 0, 0" "TraceTypeQuery1" false (Utilities|Array|MakeArray self _returnvalue_3) "None"))
          (if _returnvalue_5
            _
            (else
              (return true)))
          (else
            (bind _returnvalue_6 (Collision|BoxTraceByChannel _returnvalue (+ (* (Transformation|GetActorForwardVector _returnvalue_3) (* (Variables|Default|GetTRAVEL_DISTANCE) 2.1)) _returnvalue) (Math|Vector|MakeVector (.x _boxextent) (.y _boxextent) (* (.z _boxextent) 0.9)) "0, 0, 0" "TraceTypeQuery1" false (Utilities|Array|MakeArray self _returnvalue_3) "None"))
            (if _returnvalue_6
              _
              (else
                (return true)))))
        (return false)
        (else
          _)))
    (return false)))