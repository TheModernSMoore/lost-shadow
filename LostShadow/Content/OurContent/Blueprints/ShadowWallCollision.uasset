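; Shadow wall collision actor that rebuilds a dynamic mesh from the 2D shadow outline of a ShadowObject.
; Every Tick it searches for ShadowObject actors and reads the first one's latest points and update flag.
; When flagged, it deletes all vertices, extrudes the points as a polygon with Geometry Script, then compacts the mesh.
; An unused boolean subtract remains unconnected.
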(event EventBeginPlay)

(event Collision|EventActorBeginOverlap
  (params (OtherActor :type Actor%20Object%20Reference)))

(event EventTick
  (params (DeltaSeconds :type Float%20%28single-precision%29))
  (bind _outactors (Actor|GetAllActorsOfClass "/Game/OurContent/Blueprints/ShadowObject.ShadowObject_C"))
  (Variables|Default|Set2DPointLoctionsZY (Variables|/Game/OurContent/Blueprints/ShadowObject.ShadowObject_C|GetLatest%202D%20Point%20Locations (Utilities|Array|Get(acopy) _outactors)))
  (if (Variables|/Game/OurContent/Blueprints/ShadowObject.ShadowObject_C|GetupdatePolygon? (Utilities|Array|Get(acopy) _outactors))
    (bind _returnvalue (DynamicMeshComponent|GetDynamicMesh (Variables|DynamicMeshActor|GetDynamicMeshComponent)))
    (Utilities|IsValid (Variables|DynamicMeshActor|GetDynamicMeshComponent)
      (:Is%20Valid
        (bind _vertexidlist (Class|GeometryScriptLibraryMeshQueryFunctions|GetAllVertexIDs _returnvalue))
        (bind _returnvalue_2 (Class|GeometryScriptLibraryMeshBasicEditFunctions|DeleteVerticesfromMesh _returnvalue _vertexidlist false))
        (Class|DynamicMeshComponent|SetDynamicMesh (Variables|DynamicMeshActor|GetDynamicMeshComponent) _returnvalue_2))
      (:Is%20Not%20Valid
        _))
    (bind _returnvalue_3 (DynamicMeshComponent|GetDynamicMesh (Variables|DynamicMeshActor|GetDynamicMeshComponent)))
    (bind _returnvalue_4 (Class|GeometryScriptLibraryMeshPrimitiveFunctions|AppendSimpleExtrudePolygon :TargetMesh _returnvalue_3 :PolygonVertices (Variables|Default|Get2DPointLoctionsZY) :Debug 0))
    (bind _returnvalue_5 (Class|GeometryScriptLibraryMeshRepairFunctions|CompactMesh _returnvalue_4 0))
    (Class|DynamicMeshComponent|SetDynamicMesh (Variables|DynamicMeshActor|GetDynamicMeshComponent) _returnvalue_5)
    (Variables|Default|SetcurrentDynamicMesh _returnvalue_5)
    (DynamicMeshActor|ReleaseAllComputeMeshes)))

(fn ConstructionScript)